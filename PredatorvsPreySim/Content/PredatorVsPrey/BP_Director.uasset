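; BP_Director balances the predator-versus-prey simulation by adjusting breeding and decay to population levels.
; CountPredatorAndPrey tallies both arrays, computes their ratio and calls CalculateDirectorState.
; That function stores the average prey position, scales decay rate by population against a target, and sets each side's litter size from overcrowding and ratio checks to favour the underrepresented side.
; It also speeds up global time dilation on each calculation.
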(fn `Calculate Director State`
  (bind _targetnumberofentities (`self.TargetNumberOfEntities`))
  (bind _returnvalue (+ (`self.NumberOfPred`) (`self.NumberOfPrey`)))
  ;[1 1 1] Work out the average pos of the prey
  (`GameplayStatics.SetGlobalTimeDilation` 5.0)
  (bind _returnvalue_2 (`GameplayStatics.GetActorArrayAverageLocation` (`self.Prey`)))
  (set `self.AvgPreyPos` _returnvalue_2)
  ;[1 1 1] Work out the current ratio
  (set `self.PreyPredRatio` (/ (`self.NumberOfPrey`) (`self.NumberOfPred`)))
  ;[1 1 1] Create a higher decay rate (Rate at which things like hunger go down) if theres too many entities
  (set `self.DecayRate` (* (/ _returnvalue _targetnumberofentities) 1.0))
  ;[1 1 1] Decide if there are too many entities
  (bind _output_get (set `self.TooManyEntities` (> _returnvalue _targetnumberofentities)))
  ;[1 1 1] Work out which of prey or predator is 'winning'
  (bind _output_get_2 (set `self.TooManyPrey` (> (`self.PreyPredRatio`) (`self.TargetRatio`))))
  (if _output_get
    (if _output_get_2
      ;[1 1 1] Too many entities, too much prey
      (set `self.PreyLitterSize` 1)
      (set `self.PredLitterSize` 2)
      (else
        ;[1 1 1] Too many entities, too many predators
        (set `self.PreyLitterSize` 2)
        (set `self.PredLitterSize` 1)))
    (elif _output_get_2
      ;[1 1 1] Not enough entities, too much prey
      (set `self.PredLitterSize` 2)
      (set `self.PreyLitterSize` 1)
      (else
        ;[1 1 1] Too Many Entities, too many predators
        (set `self.PredLitterSize` 1)
        (set `self.PreyLitterSize` 3)))))

(fn `CountPredatorAndPrey`
  (bind _output_get (set `self.NumberOfPred` (`KismetArrayLibrary.Array_Length` (`self.Predator`))))
  (bind _output_get_2 (set `self.NumberOfPrey` (`KismetArrayLibrary.Array_Length` (`self.Prey`))))
  (set `self.PreyPredRatio` (/ _output_get_2 _output_get))
  (`self.Calculate Director State`))