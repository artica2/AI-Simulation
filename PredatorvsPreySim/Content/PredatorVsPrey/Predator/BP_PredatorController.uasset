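; AI controller for a predator in a predator-versus-prey ecosystem simulation, tracking age, hunger, fatigue and mating urge, and dying at their limits.
; When idle, it picks hunt, rest, mate or wander by estimating which lowers total discontent, then runs it from Tick.
; AI perception supplies prey and opposite-sex mates; females spawn litters whose speed mutates from the faster parent's.
; The BP_Director game instance supplies decay rate and litter size and tracks populations.
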(event `self.ReceiveBeginPlay`
  (`self.BeBorn`))

(event `self.ReceiveTick`
  (params (DeltaSeconds :type "Float (single-precision)"))
  (`self.UpdateNeeds` DeltaSeconds)
  (bind _isdead (`self.CheckDead`))
  (if (not _isdead)
    (switch `/Game/PredatorVsPrey/Predator/Actions` (`self.TargetAction`)
      (:`NewEnumerator0`
        (if (`KismetSystemLibrary.IsValid` (`self.Prey`))
          (`self.Hunt`)
          (else
            (set `self.TargetAction` "NewEnumerator3")
            (`KismetArrayLibrary.Array_Clear` (`|MakeArray` (`self.Prey`))))))
      (:`NewEnumerator1`
        (`KismetSystemLibrary.Delay` 5.0)
        (`self.Sleep`))
      (:`NewEnumerator2`
        (`self.Mate`))
      (:`NewEnumerator4`
        (`self.wander`))
      (:`NewEnumerator3`
        (`self.Compare Actions`)))))

(event `self.AIPerception.OnTargetPerceptionUpdated`
  (params (Actor :type "Actor Object Reference") (Stimulus :type "AIStimulus Structure"))
  (bind (_age _expirationage _strength _stimuluslocation _receiverlocation _tag _bsuccessfullysensed) (break `AIStimulus` Stimulus))
  (bind _asbp_prey (cast `/Game/PredatorVsPrey/Prey/BP_Prey` Actor)
    (:`then`
      (`self.SensePrey` _bsuccessfullysensed _asbp_prey))
    (:`CastFailed`
      (bind _asbp_predator (cast `/Game/PredatorVsPrey/Predator/BP_Predator` Actor))
      (`self.SensePred` _bsuccessfullysensed _asbp_predator))))

(fn `BeBorn`
  ;[1 1 1] Initialize variables
  (set `self.Age` 0.0)
  (set `self.Has Target` false)
  (set `self.Hunger` 100.0)
  (set `self.Fatigue` 100.0)
  (set `self.Mating Instincts` 100.0)
  (set `self.isFemale` (`KismetMathLibrary.RandomBool`))
  (set `self.TargetAction` "NewEnumerator3")
  ;[1 1 1] Update the director
  (bind _asbp_director (cast `/Game/PredatorVsPrey/BP_Director` (`GameplayStatics.GetGameInstance`)))
  (bind _asbp_predator (cast `/Game/PredatorVsPrey/Predator/BP_Predator` (`self.K2_GetPawn`)))
  (`KismetArrayLibrary.Array_Add` (`/Game/PredatorVsPrey/BP_Director.Predator` _asbp_director) _asbp_predator)
  (`/Game/PredatorVsPrey/BP_Director.CountPredatorAndPrey` _asbp_director))

(fn `CalculateInsistence`
  (params (HungerVar :type "Float (double-precision)") (FatugueVar :type "Float (double-precision)") (MatingVar :type "Float (double-precision)"))
  (returns (DiscontentVar :type "Float (double-precision)"))
  ;[1 1 1] Add the amount 'missing' from each of the desires to a discontent dummy variable
  (set `self.Discontent` 0.0)
  (set `self.Discontent` (+ (* (- 100.0 (`KismetMathLibrary.FClamp` HungerVar -5.0 100.0)) 1.0) (`self.Discontent`)))
  (set `self.Discontent` (+ (* (- 100.0 (`KismetMathLibrary.FClamp` FatugueVar -5.0 100.0)) 1.0) (`self.Discontent`)))
  (bind _output_get (set `self.Discontent` (+ (* (- 100.0 (`KismetMathLibrary.FClamp` MatingVar -5.0 100.0)) 1.0) (`self.Discontent`))))
  (return _output_get))

(fn `CheckDead`
  (returns (isDead :type Boolean))
  (bind _returnvalue (`self.K2_GetPawn`))
  ;[1 1 1] Check to see if hunger or fatigue are less than 0, or if age is greater than 500
  (if (< (`self.Hunger`) 0.0)
    _
    (elif (< (`self.Fatigue`) 0.0)
      _
      (elif (> (`self.Age`) 500.0)
        _
        (else
          (return false)))))
  ;[1 1 1] Destroy the predator and update the director accordingly
  (bind _asbp_director (cast `/Game/PredatorVsPrey/BP_Director` (`GameplayStatics.GetGameInstance`)))
  (bind _asbp_predator (cast `/Game/PredatorVsPrey/Predator/BP_Predator` _returnvalue))
  (`KismetArrayLibrary.Array_RemoveItem` (`/Game/PredatorVsPrey/BP_Director.Predator` _asbp_director) _asbp_predator)
  (`/Game/PredatorVsPrey/BP_Director.CountPredatorAndPrey` _asbp_director)
  (set `self.TargetAction` "NewEnumerator3")
  (`self.K2_DestroyActor` _returnvalue)
  (return true))

(fn `Compare Actions`
  (bind _prey (`self.Prey`))
  (bind _mating_instincts (`self.Mating Instincts`))
  (bind _fatigue (`self.Fatigue`))
  (set `self.TargetAction` "NewEnumerator4")
  (set `self.Discontent Dummy` 100.0)
  ;[1 1 1] Test sleep
  (if (not (> _fatigue 60.0))
    (bind _discontentvar (`self.CalculateInsistence` (`self.Hunger`) (+ _fatigue 50.0) (`self.Mating Instincts`)))
    (set `self.Discontent Dummy` _discontentvar)
    (set `self.TargetAction` "NewEnumerator1"))
  ;[1 1 1] Test Eat
  (bind _discontentvar_2 (`self.CalculateInsistence` (+ (`self.Hunger`) 50.0) (`self.Fatigue`) (`self.Mating Instincts`)))
  (if (< (`self.Hunger`) 60.0)
    (if (< _discontentvar_2 (`self.Discontent Dummy`))
      (cast `Actor` _prey
        (:`then`
          (if (`KismetSystemLibrary.IsValid` _prey)
            (set `self.TargetAction` "NewEnumerator0")
            (set `self.Discontent Dummy` _discontentvar_2)
            ;[1 1 1] Test mate
            (if (not (> _mating_instincts 60.0)) :!label _label
              (bind _discontentvar_3 (`self.CalculateInsistence` (`self.Hunger`) (`self.Fatigue`) (+ _mating_instincts 50.0)))
              (if (< _discontentvar_3 (`self.Discontent Dummy`))
                (cast `Actor` (`self.Other Predator`))
                (set `self.TargetAction` "NewEnumerator2")
                (set `self.Discontent Dummy` _discontentvar_3)))))
        (:`CastFailed`
          (goto _label)))
      (else
        (goto _label)))
    (else
      (goto _label))))

(fn `Hunt`
  (bind _prey (`self.Prey`))
  (bind _prey_2 (`self.Prey`))
  ;[1 1 1] Move towards the prey
  (if (`KismetSystemLibrary.IsValid` _prey)
    (bind _asactor (cast `Actor` _prey)
      (:`then`
        (`self.MoveToActor` _asactor -1.0 true true true null)
        (bind _asactor_2 (cast `Actor` self))
        (bind _asbp_prey (cast `/Game/PredatorVsPrey/Prey/BP_Prey` (`self.Prey`)))
        (bind _asactor_3 (cast `Actor` _asbp_prey))
        ;[1 1 1] Check if we are within kill range
        (if (< (`KismetMathLibrary.Vector_Distance` (`self.K2_GetActorLocation` _asactor_3) (`self.K2_GetActorLocation` _asactor_2)) 200.0)
          ;[1 1 1] Kill the prey and update the director accordingly
          (`self.K2_DestroyActor` _asactor_3)
          (set `self.Hunger` 100.0)
          (set `self.TargetAction` "NewEnumerator3")
          (`KismetArrayLibrary.Array_Clear` (`|MakeArray` _prey_2))
          (bind _asbp_director (cast `/Game/PredatorVsPrey/BP_Director` (`GameplayStatics.GetGameInstance`)))
          (bind _asbp_prey_2 (cast `/Game/PredatorVsPrey/Prey/BP_Prey` _prey_2))
          (`KismetArrayLibrary.Array_RemoveItem` (`/Game/PredatorVsPrey/BP_Director.Prey` _asbp_director) _asbp_prey_2)))
      (:`CastFailed`
        (set `self.TargetAction` "NewEnumerator3" :!label _label)))
    (else
      (goto _label))))

(fn `Mate`
  (bind _other_predator (`self.Other Predator`))
  ;[1 1 1] If our other predator exists, move towards it
  (if (`KismetSystemLibrary.IsValid` _other_predator)
    (bind _asactor (cast `Actor` _other_predator)
      (:`then`
        (`self.MoveToActor` _asactor -1.0 true true true null)
        ;[1 1 1] Test if we are within mating range
        (bind _asactor_2 (cast `Actor` self))
        (bind _asbp_predator (cast `/Game/PredatorVsPrey/Predator/BP_Predator` (`self.Other Predator`)))
        (bind _asactor_3 (cast `Actor` _asbp_predator))
        (bind _returnvalue (`self.K2_GetActorLocation` _asactor_2))
        ;[1 1 1] Only the female spawns children
        (if (< (`KismetMathLibrary.Vector_Distance` (`self.K2_GetActorLocation` _asactor_3) _returnvalue) 200.0)
          (if (`self.isFemale`)
            ;[1 1 1] Reset the mating instincts of both parents
            (bind _asbp_predator_controller (cast `/Game/PredatorVsPrey/Predator/BP_PredatorController` (`AIBlueprintHelperLibrary.GetAIController` _asbp_predator)))
            (`self.Reset Mating` _asbp_predator_controller _asbp_predator_controller)
            (`self.Reset Mating` self)
            ;[1 1 1] Spawn as many children as our director instructs
            (bind _asbp_director (cast `/Game/PredatorVsPrey/BP_Director` (`GameplayStatics.GetGameInstance`)))
            (for _ (range 1 (+ (`/Game/PredatorVsPrey/BP_Director.PredLitterSize` _asbp_director) 1))
              (`self.SpawnChild` (`KismetMathLibrary.Conv_VectorToTransform` _returnvalue) _asbp_predator_controller self)))
          (set `self.TargetAction` "NewEnumerator3")))
      (:`CastFailed`
        (set `self.TargetAction` "NewEnumerator3" :!label _label)))
    (else
      (`KismetArrayLibrary.Array_Clear` (`|MakeArray` _other_predator))
      (goto _label))))

(fn `Reset Mating`
  (params (PredController :type "/Game/PredatorVsPrey/Predator/BP_PredatorController Object Reference"))
  (set `/Game/PredatorVsPrey/Predator/BP_PredatorController.Mating Instincts` 100.0 PredController))

(fn `SensePred`
  (params (HasSensed :type Boolean) (Pred :type "/Game/PredatorVsPrey/Predator/BP_Predator Object Reference"))
  ;[1 1 1] Check if we are forgetting or learning about a predator
  (if HasSensed
    ;[1 1 1] Check the other predator is both ready to mate and of the opposite gender
    (bind _asbp_predator_controller (cast `/Game/PredatorVsPrey/Predator/BP_PredatorController` (`AIBlueprintHelperLibrary.GetAIController` Pred)))
    (if (== (`self.isFemale`) (`/Game/PredatorVsPrey/Predator/BP_PredatorController.isFemale` _asbp_predator_controller))
      _
      (elif true
        (if (not (> (`/Game/PredatorVsPrey/Predator/BP_PredatorController.Mating Instincts` _asbp_predator_controller) 60.0))
          (set `self.Other Predator` Pred))))
    (else
      (`KismetArrayLibrary.Array_Clear` (`|MakeArray` (`self.Other Predator`))))))

(fn `SensePrey`
  (params (HasSensed :type Boolean) (Prey :type "/Game/PredatorVsPrey/Prey/BP_Prey Object Reference"))
  (if HasSensed
    (set `self.Prey` Prey)
    (else
      (`KismetArrayLibrary.Array_Clear` (`|MakeArray` (`self.Prey`))))))

(fn `Sleep`
  (set `self.Fatigue` (+ 50.0 (`self.Fatigue`)))
  (set `self.TargetAction` "NewEnumerator3"))

(fn `SpawnChild`
  (params (Location :type "Transform Structure") (Father :type "/Game/PredatorVsPrey/Predator/BP_PredatorController Object Reference") (Mother :type "/Game/PredatorVsPrey/Predator/BP_PredatorController Object Reference"))
  ;[1 1 1] Get Parents Speed
  (bind _asbp_predator (cast `/Game/PredatorVsPrey/Predator/BP_Predator` (`self.K2_GetPawn` Father)))
  (bind _speed (`/Game/PredatorVsPrey/Predator/BP_Predator.Get Speed` _asbp_predator))
  (bind _asbp_predator_2 (cast `/Game/PredatorVsPrey/Predator/BP_Predator` (`self.K2_GetPawn` Mother)))
  (bind _speed_2 (`/Game/PredatorVsPrey/Predator/BP_Predator.Get Speed` _asbp_predator_2))
  ;[1 1 1] Spawn the predator and set the speed
  (bind _returnvalue (`|SpawnActorFromClass` "/Game/PredatorVsPrey/Predator/BP_Predator.BP_Predator_C" Location "Undefined" "MultiplyWithRoot" null null))
  (if (> _speed _speed_2)
    (bind _returnvalue_2 (/ _speed 10.0))
    (`/Game/PredatorVsPrey/Predator/BP_Predator.Set Speed` _returnvalue (`KismetMathLibrary.RandomFloatInRange` (- _speed _returnvalue_2) (+ _returnvalue_2 _speed)))
    (else
      (bind _returnvalue_3 (/ _speed_2 10.0))
      (`/Game/PredatorVsPrey/Predator/BP_Predator.Set Speed` _returnvalue (`KismetMathLibrary.RandomFloatInRange` (+ _speed_2 _returnvalue_3) (- _speed_2 _returnvalue_3)))))
  (bind _asbp_predator_controller (cast `/Game/PredatorVsPrey/Predator/BP_PredatorController` (`Pawn.GetController` _returnvalue)))
  (`self.BeBorn` _asbp_predator_controller)
  (return))

(fn `UpdateNeeds`
  (params (Time :type "Float (double-precision)"))
  ;[1 1 1] Update each variable using time x the directors decay rate
  (bind _asbp_director (cast `/Game/PredatorVsPrey/BP_Director` (`GameplayStatics.GetGameInstance`)))
  (bind _returnvalue (* Time (`/Game/PredatorVsPrey/BP_Director.DecayRate` _asbp_director)))
  (set `self.Age` (+ _returnvalue (`self.Age`)))
  (set `self.Hunger` (- (`self.Hunger`) _returnvalue))
  (set `self.Fatigue` (- (`self.Fatigue`) _returnvalue))
  (set `self.Mating Instincts` (- (`self.Mating Instincts`) (* _returnvalue 2.0)))
  (set `self.DeltaTime` Time)
  ;[1 1 1] Make sure the controller stays attatched to the controlled
  (`self.K2_SetActorLocation` (`self.K2_GetActorLocation` (`self.K2_GetPawn`))))

(fn `UserConstructionScript`)

(fn `wander`
  (if (not (`self.Has Target`))
    ;[1 1 1] If we dont have a wander location, choose a new one
    (bind _randomlocation (`NavigationSystemV1.K2_GetRandomLocationInNavigableRadius` (`self.K2_GetActorLocation` (`self.K2_GetPawn`)) (`self.Radius`) null null))
    (set `self.Has Target` true)
    (bind _output_get (set `self.target` _randomlocation)))
  ;[1 1 1] Move towards the target location, if we get there (or within 100 units of there), wipe clean our target so a new one will be picked next frame
  (`self.MoveToLocation` _output_get -1.0 true true false true null)
  (bind _asactor (cast `Actor` self))
  (if (< (`KismetMathLibrary.Vector_Distance` (`self.target`) (`self.K2_GetActorLocation` _asactor)) 100.0)
    (set `self.Has Target` false)
    (set `self.TargetAction` "NewEnumerator3")))