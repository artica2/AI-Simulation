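; AI controller for prey in a predator-vs-prey simulation, running BT_PreyTree and registering each newborn with the BP_Director game instance.
; Tick decays hunger and energy at the director's rate, counts down mating cooldown, and snaps the controller to its pawn.
; AI perception writes blackboard targets: opposite-sex prey ready to mate, the nearest sensed predator to flee, and food, clearing each when sensing is lost.
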(event `self.ReceiveBeginPlay`
  (`self.BeBorn`))

(event `self.ReceiveTick`
  (params (DeltaSeconds :type "Float (single-precision)"))
  (`self.UpdateNeeds` DeltaSeconds)
  ;[1 1 1] Make sure controller and controlled stay together
  (`self.K2_SetActorLocation` (`self.K2_GetActorLocation` (`self.K2_GetPawn`))))

(event `self.AIPerception.OnTargetPerceptionUpdated`
  (params (Actor :type "Actor Object Reference") (Stimulus :type "AIStimulus Structure"))
  (bind (_age _expirationage _strength _stimuluslocation _receiverlocation _tag _bsuccessfullysensed) (break `AIStimulus` Stimulus))
  ;[1 1 1] Make sure not sensing itself
  (if (not (== (`self.K2_GetPawn`) Actor))
    (bind _asbp_prey (cast `/Game/PredatorVsPrey/Prey/BP_Prey` Actor)
      (:`then`
        (`self.Sense Prey` _bsuccessfullysensed _asbp_prey))
      (:`CastFailed`
        (bind _asbp_predator (cast `/Game/PredatorVsPrey/Predator/BP_Predator` Actor)
          (:`then`
            (`self.Sense Predator` _bsuccessfullysensed _asbp_predator))
          (:`CastFailed`
            (bind _asbp_food (cast `/Game/PredatorVsPrey/Food/BP_Food` Actor))
            (`self.Sense Food` _bsuccessfullysensed _asbp_food)))))))

(fn `BeBorn`
  (bind _blackboard (`self.Blackboard`))
  ;[1 1 1] Initialize variables
  (`self.RunBehaviorTree` "/Game/PredatorVsPrey/Prey/BT_PreyTree.BT_PreyTree")
  (`BlackboardComponent.SetValueAsFloat` _blackboard "Hunger" 100.0)
  (`BlackboardComponent.SetValueAsFloat` _blackboard "Energy" 100.0)
  (`BlackboardComponent.SetValueAsBool` _blackboard "isFemale" (`KismetMathLibrary.RandomBool`))
  (`BlackboardComponent.SetValueAsFloat` _blackboard "MatingCooldown" 40.0)
  ;[1 1 1] Add the new prey to the director
  (bind _asbp_director (cast `/Game/PredatorVsPrey/BP_Director` (`GameplayStatics.GetGameInstance`)))
  (bind _asbp_prey (cast `/Game/PredatorVsPrey/Prey/BP_Prey` (`self.K2_GetPawn`)))
  (`KismetArrayLibrary.Array_Add` (`/Game/PredatorVsPrey/BP_Director.Prey` _asbp_director) _asbp_prey)
  (`/Game/PredatorVsPrey/BP_Director.CountPredatorAndPrey` _asbp_director))

(fn `Sense Food`
  (params (HasSensed :type Boolean) (Food :type "/Game/PredatorVsPrey/Food/BP_Food Object Reference"))
  (bind _blackboard (`self.Blackboard`))
  (if HasSensed
    (`BlackboardComponent.SetValueAsObject` _blackboard "Food" Food)
    (else
      (`BlackboardComponent.ClearValue` _blackboard "Food"))))

(fn `Sense Predator`
  (params (HasSensed :type Boolean) (Predator :type "/Game/PredatorVsPrey/Predator/BP_Predator Object Reference"))
  (bind _blackboard (`self.Blackboard`))
  (bind _returnvalue (`BlackboardComponent.GetValueAsObject` _blackboard "Predator"))
  (bind _returnvalue_2 (`self.K2_GetActorLocation` (`self.K2_GetPawn`)))
  (if HasSensed
    ;[1 1 1] Check if the newly sensed predator is closer than the currently watched predator, if so overwrite, if not don't overwrite (This is so the prey will flee the nearest predator)
    (if (`KismetSystemLibrary.IsValid` _returnvalue)
      (bind _asbp_predator (cast `/Game/PredatorVsPrey/Predator/BP_Predator` _returnvalue))
      (bind _asbp_predator_2 (cast `/Game/PredatorVsPrey/Predator/BP_Predator` Predator))
      (if (not (< (`KismetMathLibrary.VSize` (- _returnvalue_2 (`self.K2_GetActorLocation` _asbp_predator))) (`KismetMathLibrary.VSize` (- _returnvalue_2 (`self.K2_GetActorLocation` _asbp_predator_2)))))
        (`BlackboardComponent.SetValueAsObject` _blackboard "Predator" Predator :!label _label))
      (else
        (goto _label)))
    (else
      (`BlackboardComponent.ClearValue` _blackboard "Predator"))))

(fn `Sense Prey`
  (params (HasSensed :type Boolean) (Prey :type "/Game/PredatorVsPrey/Prey/BP_Prey Object Reference"))
  (bind _blackboard (`self.Blackboard`))
  (bind _returnvalue (`AIBlueprintHelperLibrary.GetBlackboard` (`AIBlueprintHelperLibrary.GetAIController` Prey)))
  ;[1 1 1] If we are forgetting, clear OtherPrey
  (if HasSensed
    ;[1 1 1] Make sure the prey is both ready to mate and of the opposite gender
    (if (== (`BlackboardComponent.GetValueAsBool` _returnvalue "isFemale") (`BlackboardComponent.GetValueAsBool` _blackboard "isFemale"))
      _
      (elif (== (`BlackboardComponent.GetValueAsBool` _returnvalue "CanMate") true)
        (`BlackboardComponent.SetValueAsObject` _blackboard "OtherPrey" Prey)))
    (else
      (`BlackboardComponent.ClearValue` (`AIBlueprintHelperLibrary.GetBlackboard` null) "OtherPrey"))))

(fn `UpdateNeeds`
  (params (Time :type "Float (double-precision)"))
  (bind _blackboard (`self.Blackboard`))
  (bind _blackboard_2 (`self.Blackboard`))
  (bind _blackboard_3 (`self.Blackboard`))
  (bind _blackboard_4 (`self.Blackboard`))
  (bind _returnvalue (- (`BlackboardComponent.GetValueAsFloat` _blackboard_4 "MatingCooldown") Time))
  ;[1 1 1] Get the decay rate
  (bind _asbp_director (cast `/Game/PredatorVsPrey/BP_Director` (`GameplayStatics.GetGameInstance`)))
  (bind _returnvalue_2 (* Time (`/Game/PredatorVsPrey/BP_Director.DecayRate` _asbp_director)))
  ;[1 1 1] Update hunger
  (`BlackboardComponent.SetValueAsFloat` _blackboard_2 "Hunger" (- (`BlackboardComponent.GetValueAsFloat` _blackboard_2 "Hunger") _returnvalue_2))
  ;[1 1 1] Update Energy
  (`BlackboardComponent.SetValueAsFloat` _blackboard_3 "Energy" (- (`BlackboardComponent.GetValueAsFloat` _blackboard_3 "Energy") _returnvalue_2))
  ;[1 1 1] Upate mating instict
  (`BlackboardComponent.SetValueAsFloat` _blackboard_4 "MatingCooldown" _returnvalue)
  ;[1 1 1] Check whether the prey can mate
  (if (< _returnvalue 0.0)
    (`BlackboardComponent.SetValueAsBool` _blackboard "CanMate" true)
    (else
      (`BlackboardComponent.SetValueAsBool` _blackboard "CanMate" false))))

(fn `UserConstructionScript`)